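; BP_Guard is an AI guard that arms itself with an assault hitscan weapon when play begins.
; It spawns BP_Hitscan_Assult at its own transform, then overrides it for infinite ammo, a set attack delay and zeroed recoil and spread growth.
; The configured weapon is then equipped through the CombatComponent; the graph holds no other behavior.
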(event `self.ReceiveBeginPlay`
  (bind _returnvalue (`|SpawnActorFromClass` "/Game/ProjectFile/Actor/Weapon/Hitscan/BP_Hitscan_Assult.BP_Hitscan_Assult_C" (`self.GetTransform`) "Undefined" "SelectDefaultAtRuntime" null null))
  (`|ExecutionSequence`
    (:`then_0`
      (set `Gun.bInfinityAmmo` true _returnvalue)
      (set `Gun.AttackDelay` 0.5 _returnvalue)
      (set `Gun.MaxRecoilPitch` 0.0 _returnvalue)
      (set `Gun.MaxRecoilYaw` 0.0 _returnvalue)
      (set `Gun.MinRecoilPitch` 0.0 _returnvalue)
      (set `Gun.MinRecoilYaw` 0.0 _returnvalue)
      (set `Gun.SpreadPerTime` 0.0 _returnvalue))
    (:`then_1`
      (`CombatComponent.EquipWeapon` (`self.CombatComponent`) _returnvalue))))

(fn `UserConstructionScript`)