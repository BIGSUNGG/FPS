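; BP_Spawner is an actor that spawns a creature of a BP_KraverPlayer class whenever it takes damage.
; AnyDamage calls SpawnCreature, which first destroys the previously spawned creature if it is still valid.
; It then casts the class to BP_KraverPlayer, spawns it a fixed distance in front of the spawner with matching rotation and scale, and stores it in CurSpawnCreature for the next replacement.
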(event `self.ReceiveActorBeginOverlap`
  (params (OtherActor :type "Actor Object Reference")))

(event `self.ReceiveTick`
  (params (DeltaSeconds :type "Float (single-precision)")))

(event `self.ReceiveAnyDamage`
  (params (Damage :type "Float (single-precision)") (DamageType :type "DamageType Object Reference") (InstigatedBy :type "Controller Object Reference") (DamageCauser :type "Actor Object Reference"))
  (`self.Spawn Creature`))

(fn `Spawn Creature`
  (bind _curspawncreature (`self.CurSpawnCreature`))
  (`|ExecutionSequence`
    (:`then_0`
      (`/Engine/EditorBlueprintResources/StandardMacros.IsValid` _curspawncreature
        (:`Is Valid`
          (`self.K2_DestroyActor` _curspawncreature))))
    (:`then_1`
      (bind _asbp_kraver_player (castclass `/Game/ProjectFile/Creature/BP_KraverPlayer` "/Game/ProjectFile/Creature/BP_KraverPlayer.BP_KraverPlayer_C"))
      (bind _returnvalue (`|SpawnActorFromClass` _asbp_kraver_player (`KismetMathLibrary.MakeTransform` (+ (.location (`self.GetTransform`)) (* (`self.GetActorForwardVector`) 200.0)) (.rotation (`self.GetTransform`)) (.scale (`self.GetTransform`))) "Undefined" "SelectDefaultAtRuntime" null null))
      (set `self.CurSpawnCreature` _returnvalue))))

(fn `UserConstructionScript`)