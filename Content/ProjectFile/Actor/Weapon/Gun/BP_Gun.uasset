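; BP_Gun is a gun weapon Blueprint that wires up reload and muzzle effect parts in its Construction Script.
; It adds WeaponReload to WeaponComponents and assigns it first- and third-person assault rifle reload montages.
; It registers the mesh and fire effect by name in WeaponPrimitiveInfo, then snaps the effect to the muzzle socket with a rotation offset.
; The Event Graph holds no logic.
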(event `self.ReceiveBeginPlay`)

(fn `UserConstructionScript`
  (bind _weaponreload (`self.WeaponReload`))
  (bind _weaponprimitiveinfo (`self.WeaponPrimitiveInfo`))
  (`|ExecutionSequence`
    (:`then_0`
      (`KismetArrayLibrary.Array_Add` (`self.WeaponComponents`) _weaponreload))
    (:`then_1`
      (set `WeaponReloadComponent.ReloadMontageFpp` "/Game/InfimaGames/AnimatedLowPolyWeapons/Art/Characters/Animations/ARs/AM_FP_PCH_AR_01_Reload.AM_FP_PCH_AR_01_Reload" _weaponreload)
      (set `WeaponReloadComponent.ReloadMontageTpp` "/Game/InfimaGames/AnimatedLowPolyWeapons/Art/Characters/Animations/ARs/AM_TP_CH_AR_01_Reload.AM_TP_CH_AR_01_Reload" _weaponreload)
      (`BlueprintMapLibrary.Map_Add` _weaponprimitiveinfo "Root" (`self.WeaponMesh`))
      (`BlueprintMapLibrary.Map_Add` _weaponprimitiveinfo "FireEffect" (`self.FireEffect`))
      (`SceneComponent.K2_AttachToComponent` (`self.FireEffect`) (`self.WeaponMesh`) "SOCKET_Muzzle" "SnapToTarget" "SnapToTarget" "SnapToTarget" true)
      (`SceneComponent.K2_SetRelativeRotation` (`self.FireEffect`) (struct :`Yaw` 90.0) false false))))