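; BP_RocketLauncher is a rocket launcher gun Blueprint that sets up its weapon components in the construction script.
; It registers the weapon mesh and fire effect in the WeaponPrimitiveInfo map under named keys.
; The fire effect is snapped to the mesh's muzzle socket and given a fixed rotation offset.
; The event graph holds only empty events, so no firing logic lives in these graphs.
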(fn `UserConstructionScript`
  (`BlueprintMapLibrary.Map_Add` (`self.WeaponPrimitiveInfo`) "Root" (`self.WeaponMesh`))
  (`BlueprintMapLibrary.Map_Add` (`self.WeaponPrimitiveInfo`) "FireEffect" (`self.FireEffect`))
  (`SceneComponent.K2_AttachToComponent` (`self.FireEffect`) (`self.WeaponMesh`) "SOCKET_Muzzle" "SnapToTarget" "SnapToTarget" "SnapToTarget" true)
  (`SceneComponent.K2_SetRelativeRotation` (`self.FireEffect`) (struct :`Yaw` 90.0) false false))