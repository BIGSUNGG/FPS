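; BP_Attaker is a creature Blueprint that arms itself with an assault rifle and starts attacking when play begins.
; BeginPlay spawns BP_AssultRifle at its own transform, then gives it infinite ammo and a fixed attack delay.
; It sets the rifle as CanInteractWeapon and calls the equip and attack button functions directly, with no release call.
; Nodes zeroing the rifle's recoil and spread are unconnected and never run.
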(event `self.ReceiveBeginPlay`
  (`parent.ReceiveBeginPlay`)
  (bind _returnvalue (`|SpawnActorFromClass` "/Game/ProjectFile/Weapon/Gun/BP_AssultRifle.BP_AssultRifle_C" (`self.GetTransform`) "Undefined" "SelectDefaultAtRuntime" null null))
  (`|ExecutionSequence`
    (:`then_0`
      (set `Gun.bInfinityAmmo` true _returnvalue)
      (set `Weapon.AttackDelay` 0.5 _returnvalue))
    (:`then_1`
      (set `self.CanInteractWeapon` _returnvalue)
      (`self.EquipButtonPressed`)
      (`self.AttackButtonPressed`))))

(fn `UserConstructionScript`
  (`parent.UserConstructionScript`))