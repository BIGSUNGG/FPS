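; BP_Soldier is a creature Blueprint for a soldier that arms itself with an assault rifle at BeginPlay.
; It spawns a BP_AssultRifle at its own transform, gives it infinite ammo and a fixed attack delay, then equips it through CombatComponent.
; Nodes that would zero the rifle's recoil and spread are present but unconnected, so they never run.
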(event `self.ReceiveBeginPlay`
  (bind _asbp_assult_rifle (castclass `/Game/ProjectFile/Weapon/Gun/BP_AssultRifle` "/Game/ProjectFile/Weapon/Gun/BP_AssultRifle.BP_AssultRifle_C"))
  (bind _returnvalue (`|SpawnActorFromClass` _asbp_assult_rifle (`self.GetTransform`) "Undefined" "OverrideRootScale" null null))
  (`|ExecutionSequence`
    (:`then_0`
      (set `Gun.bInfinityAmmo` true _returnvalue)
      (set `Weapon.AttackDelay` 0.5 _returnvalue))
    (:`then_1`
      (`CombatComponent.EquipWeapon` (`self.CombatComponent`) _returnvalue))))

(fn `UserConstructionScript`)