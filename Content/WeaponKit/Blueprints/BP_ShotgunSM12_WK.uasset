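; Shotgun weapon Blueprint for the SM12 in WeaponKit, adding multi-pellet fire and visible external shells to its parent weapon class.
; ExecuteBulletFire repeats the parent's bullet fire in a loop sized by NumPelletsInShell, so pellets reuse the parent's shot logic.
; A notify event shows or hides the three external shell meshes together.
; GetExternalShellMeshes fills an array with those meshes plus the reload shell mesh.
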(event `/Game/WeaponKit/Blueprints/Classes/BP_WeaponActorBase_WK.Notify_ExternalShellToggle`
  (params (bOn :type Boolean))
  (`SceneComponent.SetVisibility` (`self.ExtShellMesh0`) bOn false)
  (`SceneComponent.SetVisibility` (`self.ExtShellMesh1`) bOn false)
  (`SceneComponent.SetVisibility` (`self.ExtShellMesh2`) bOn false))

(fn `ExecuteBulletFire`
  (for _ (range (+ (`KismetMathLibrary.Max` (- (`self.NumPelletsInShell`) 1) 1) 1))
    (`parent.ExecuteBulletFire`)))

(fn `GetExternalShellMeshes`
  (params (MeshArray :type "Array of MeshComponent Object Reference (by ref)"))
  (returns (NumMeshes :type Integer))
  (bind _mesharray (`local.MeshArray`))
  (`KismetArrayLibrary.Array_Clear` MeshArray)
  (`KismetArrayLibrary.Array_Add` _mesharray (`self.ExtShellMesh0`))
  (`KismetArrayLibrary.Array_Add` _mesharray (`self.ExtShellMesh1`))
  (`KismetArrayLibrary.Array_Add` _mesharray (`self.ExtShellMesh2`))
  (bind _returnvalue (`KismetArrayLibrary.Array_Add` _mesharray (`self.ReloadShellMesh`)))
  (return (+ _returnvalue 1)))

(fn `UserConstructionScript`
  (`parent.UserConstructionScript`))