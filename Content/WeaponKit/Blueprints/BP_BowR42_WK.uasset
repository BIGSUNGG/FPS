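; BP_BowR42_WK is a WeaponKit bow weapon that fires arrows as projectile proxies with a slight upward tilt.
; Construction attaches arrow, pointer and scope meshes to body sockets, and getters expose them to the parent weapon logic.
; The arrow serves as the external shell, its visibility following the chambered round and shell display settings.
; With FOV materials active, scope and laser bounds are enlarged.
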(event `self.Notify_ExternalShellToggle`
  (params (bOn :type Boolean))
  (`SceneComponent.SetVisibility` (`self.ArrowMesh`) (and bOn (`self.HasChamberedRound`)) false))

(event `self.Notify_FireBullet`
  (if (`self.HasChamberedRound`)
    (`self.SpawnProjectileProxy` false (1.0 0.0 0.05) (20.0 0.0 -5.0) (`.TraceBulletsFromController_65_CE3C8C754782A3D551388EA8D1252A65` (break `/Game/WeaponKit/Blueprints/Classes/FWeaponState_WK` (`self.State`))) 20.0))
  (`parent.Notify_FireBullet`))

(fn `ApplyState`
  (params (NewState :type "/Game/WeaponKit/Blueprints/Classes/FWeaponState_WK Structure") (bForce :type Boolean))
  (`parent.ApplyState` NewState bForce)
  (`SceneComponent.SetVisibility` (`self.ArrowMesh`) (and (`self.HasChamberedRound`) (`.ShowExternalShells_46_D60D0ED54D90F785C0C531A48D58694D` (break `/Game/WeaponKit/Blueprints/Classes/FWeaponSettings_WK` (`self.Settings`)))) false))

(fn `GetExternalShellMeshes`
  (params (MeshArray :type "Array of MeshComponent Object Reference (by ref)"))
  (returns (NumMeshes :type Integer))
  (bind _returnvalue (`KismetArrayLibrary.Array_Add` MeshArray (`self.ArrowMesh`)))
  (return (+ _returnvalue 1)))

(fn `GetPointerLaserMesh`
  (returns (Mesh :type "StaticMeshComponent Object Reference"))
  (return (`self.PointerLaserMesh`)))

(fn `GetPointerMesh`
  (returns (Mesh :type "StaticMeshComponent Object Reference"))
  (return (`self.PointerMesh`)))

(fn `GetScopeMesh`
  (returns (Mesh :type "StaticMeshComponent Object Reference"))
  (return (`self.ScopeMesh`)))

(fn `SetupWeaponFovMaterials`
  (params (WeaponMainMat :type "MaterialInterface Object Reference") (WeaponColorSelectMat :type "MaterialInterface Object Reference") (WeaponGlassMat :type "MaterialInterface Object Reference") (WeaponScreenMat :type "MaterialInterface Object Reference") (WeaponLaserMat :type "MaterialInterface Object Reference") (BulletMat :type "MaterialInterface Object Reference"))
  (`parent.SetupWeaponFovMaterials` WeaponMainMat WeaponColorSelectMat WeaponGlassMat WeaponScreenMat WeaponLaserMat BulletMat)
  (if (`self.HasFovMaterials`)
    (`PrimitiveComponent.SetBoundsScale` (`self.ScopeMesh`) 4.0)
    (`PrimitiveComponent.SetBoundsScale` (`self.PointerLaserMesh`) 4.0)))

(fn `UserConstructionScript`
  (`/Game/WeaponKit/Blueprints/Classes/BPFL_WeaponKitUtils.AttachArrow` (`self.GetBodyMesh`) (`self.ArrowMesh`))
  (`/Game/WeaponKit/Blueprints/Classes/BPFL_WeaponKitUtils.AttachPointer` (`self.GetBodyMesh`) (`self.PointerMesh`))
  (`/Game/WeaponKit/Blueprints/Classes/BPFL_WeaponKitUtils.AttachScope` (`self.GetBodyMesh`) (`self.ScopeMesh`))
  (`parent.UserConstructionScript`))