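; Base physics projectile for WeaponKit weapons that launches, plays sounds, spawns hit decals and self-destructs on timeout or optionally on impact.
; BeginPlay applies a launch impulse plus weighted instigator velocity and copies the owning weapon's skin material and color.
; Hits can attach it to the struck component or closest character bone with randomized, surface-aligned rotation, notifying the weapon.
; Children react through OnAttachedToActor, and decal fade follows the remaining lifetime.
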(event `OnAttachedToActor`
  (params (OtherComponent :type "SceneComponent Object Reference") (OtherActor :type "Actor Object Reference"))
  ;[1 1 1] Used in Child classes to react to attachment.
)

(event `self.ReceiveBeginPlay`
  (`|ExecutionSequence`
    (:`then_0`
      ;[1 1 1] Launch Projectile
      (`PrimitiveComponent.SetSimulatePhysics` (`self.ProjectileSphere`) true)
      (`PrimitiveComponent.AddImpulse` (`self.ProjectileSphere`) (`self.CalculateLaunchImpulse`) "None" true)
      (`PrimitiveComponent.SetPhysicsLinearVelocity` (`self.ProjectileSphere`) (`self.CalculateInheritedVelocity`) true "None")
      (`self.PlayLaunchSound`))
    (:`then_1`
      ;[1 1 1] Match material to owning weapon
      (set `self.OwningWeapon` (`self.GetOwningWeapon`))
      (bind _owningweapon (`self.OwningWeapon`)
        (:`then`
          (bind (_materialinst _colorparam _color) (`self.GetOwnerMaterialParams` _owningweapon))
          (bind _returnvalue (`PrimitiveComponent.CreateDynamicMaterialInstance` (`self.ProjectileSkelMesh`) 0 _materialinst "None"))
          (`MaterialInstanceDynamic.SetVectorParameterValue` _returnvalue _colorparam _color))
        (:`else`)))
    (:`then_2`
      ;[1 1 1] Manage Lifetime
      (if (> (`self.Lifetime`) 0.01)
        (bind _returnvalue_2 (`KismetSystemLibrary.K2_SetTimerDelegate` (delegate `OnLifetimeEnd`) (`self.Lifetime`) false 0.1))
        (set `self.LifetimeTimerHandle` _returnvalue_2)))))

(event `self.ProjectileSphere.OnComponentHit`
  (params (HitComponent :type "PrimitiveComponent Object Reference") (OtherActor :type "Actor Object Reference") (OtherComp :type "PrimitiveComponent Object Reference") (NormalImpulse :type "Vector Structure") (Hit :type "HitResult Structure (by ref)"))
  (bind _lifetimetimerhandle (`self.LifetimeTimerHandle`))
  ;[1 1 1] Projectile collision, attachment and FX
  (`|ExecutionSequence`
    (:`then_0`
      (if (and (`self.bShouldAttachOnHit`) (not (`self.bIsAttachedToActor`)))
        (if (not (`KismetMathLibrary.ClassIsChildOf` (`GameplayStatics.GetObjectClass` OtherActor) "BP_ProjectileActorBase_WK_C"))
          (`self.AttachToActor` OtherComp OtherActor Hit)
          (`self.OnAttachedToActor` OtherComp OtherActor)
          (bind _owningweapon (`self.OwningWeapon`)
            (:`then`
              (`/Game/WeaponKit/Blueprints/Classes/BP_WeaponActorBase_WK.Notify_ProjectileHit` _owningweapon OtherComp (`/Game/WeaponKit/Blueprints/Classes/BPFL_WeaponKitUtils.GetHitSurface` Hit) (`self.bIsAttachedToActor`)))
            (:`else`)))))
    (:`then_1`
      (bind _hitdecal (`self.HitDecal`)
        (:`then`
          (bind _returnvalue (`|SpawnActorFromClass` _hitdecal (`self.CalculateDecalTransform` Hit) "AlwaysSpawn" "OverrideRootScale" null null))
          (bind _output_get (set `self.LastSpawnedDecal` _returnvalue))
          (if (`|EnumEquality` (`SceneComponent.Mobility` OtherComp) "Movable")
            (`self.K2_AttachToComponent` _output_get OtherComp "None" "KeepWorld" "KeepWorld" "KeepWorld" true)
            (`self.K2_AttachToComponent` (`self.LastSpawnedDecal`) OtherComp "None" "KeepWorld" "KeepWorld" "KeepWorld" true))
          (if (`KismetSystemLibrary.K2_IsValidTimerHandle` _lifetimetimerhandle)
            (`DecalComponent.SetFadeOut` (`DecalActor.Decal` (`self.LastSpawnedDecal`)) (`KismetSystemLibrary.K2_GetTimerRemainingTimeHandle` _lifetimetimerhandle) 5.0 true)))
        (:`else`)))
    (:`then_2`
      (`GameplayStatics.PlaySoundAtLocation` (`self.HitSound`) (`.ImpactPoint` (`GameplayStatics.BreakHitResult` Hit)) (struct) 1.0 1.0 0.0 "/Game/WeaponKit/FX/SA_Default_WK.SA_Default_WK" null null))
    (:`then_3`
      (if (`self.bShouldDestroyOnHit`)
        (`self.K2_DestroyActor`)))))

(event `OnLifetimeEnd`
  ;[1 1 1] Manage Lifetime
  (`self.K2_DestroyActor`))

(fn `AttachToActor`
  (params (OtherComponent :type "SceneComponent Object Reference") (OtherActor :type "Actor Object Reference") (HitResult :type "HitResult Structure (by ref)"))
  (locals (ProjectedSinkNormal :type "Vector Structure" :default (0.0 0.0 0.0)) (RandomizeRot :type "Rotator Structure" :default (struct)) (AttachToComp :type "SceneComponent Object Reference") (AttachToSocket :type Name :default "None"))
  (bind (_bblockinghit _binitialoverlap _time _distance _location _impactpoint _normal) (`GameplayStatics.BreakHitResult` HitResult))
  (bind _projectilesphere (`self.ProjectileSphere`))
  (bind _projectedsinknormal (`local.ProjectedSinkNormal`))
  (bind _returnvalue (`SceneComponent.GetRightVector` (`self.ProjectileSphere`)))
  (`|ExecutionSequence`
    (:`then_0`
      (`PrimitiveComponent.SetSimulatePhysics` (`self.ProjectileSphere`) false)
      (set `local.AttachToComp` OtherComponent)
      (bind _ascharacter (cast `Character` OtherActor))
      (set `local.AttachToComp` (`Character.Mesh` _ascharacter)))
    (:`then_1`
      (bind _asskeletal_mesh_component (cast `SkeletalMeshComponent` (`local.AttachToComp`)))
      (set `local.AttachToSocket` (`.ReturnValue` (`SkinnedMeshComponent.FindClosestBone_K2` _asskeletal_mesh_component _impactpoint 0.0 true))))
    (:`then_2`
      (bind _returnvalue_2 (`SceneComponent.K2_AttachToComponent` (`self.ProjectileSphere`) (`local.AttachToComp`) (`local.AttachToSocket`) "KeepWorld" "KeepWorld" "KeepWorld" true))
      (set `self.bIsAttachedToActor` _returnvalue_2)
      (`PrimitiveComponent.SetCollisionEnabled` (`self.ProjectileSphere`) "NoCollision"))
    (:`then_3`
      (set `local.RandomizeRot` (`KismetMathLibrary.MakeRotator` (* (`KismetMathLibrary.RandomFloatInRange` -1.0 1.0) (`self.RandomizeRoll`)) 0.0 (* (`KismetMathLibrary.RandomFloatInRange` -1.0 1.0) (`self.RandomizeYaw`)))))
    (:`then_4`
      (set `local.ProjectedSinkNormal` (`KismetMathLibrary.NegateVector` (`KismetMathLibrary.ProjectVectorOnToPlane` _normal _returnvalue)))
      (`SceneComponent.K2_SetWorldRotation` _projectilesphere (`KismetMathLibrary.ComposeRotators` (`local.RandomizeRot`) (`KismetMathLibrary.SelectRotator` (`SceneComponent.K2_GetComponentRotation` (`self.ProjectileSphere`)) (`KismetMathLibrary.MakeRotationFromAxes` _projectedsinknormal _returnvalue (`KismetMathLibrary.Cross_VectorVector` _projectedsinknormal _returnvalue)) (`KismetMathLibrary.Vector_IsZero` (`local.ProjectedSinkNormal`)))) false true)
      (`SceneComponent.K2_SetWorldLocation` _projectilesphere _impactpoint false true))))

(fn `CalculateDecalTransform`
  (params (Hit :type "HitResult Structure (by ref)"))
  (returns (ReturnValue :type "Transform Structure"))
  (bind (_bblockinghit _binitialoverlap _time _distance _location _impactpoint _normal) (`GameplayStatics.BreakHitResult` Hit))
  (return (`KismetMathLibrary.MakeTransform` (`KismetMathLibrary.SelectVector` (.location (`self.GetTransform`)) _location (`self.bIsAttachedToActor`)) (`KismetMathLibrary.ComposeRotators` (struct :`Yaw` 90.0 :`Roll` -90.0) (`KismetMathLibrary.SelectRotator` (.rotation (`self.GetTransform`)) (`KismetMathLibrary.Conv_VectorToRotator` (`KismetMathLibrary.NegateVector` _normal)) (`self.bIsAttachedToActor`))) (`self.HitDecalScale`))))

(fn `CalculateInheritedVelocity`
  (returns (Result :type "Vector Structure"))
  (locals (InstigatorTR :type "Transform Structure"))
  (bind _inheritvelocity (`self.InheritVelocity`))
  (bind _instigator (`self.Instigator`)
    (:`then`
      (bind _output_get (set `local.InstigatorTR` (`self.GetTransform` _instigator)))
      (return (`KismetMathLibrary.TransformDirection` (`local.InstigatorTR`) (`KismetMathLibrary.MakeVector` (* (.x (`KismetMathLibrary.InverseTransformDirection` _output_get (`self.GetVelocity` _instigator))) _inheritvelocity) (* (.y (`KismetMathLibrary.InverseTransformDirection` _output_get (`self.GetVelocity` _instigator))) (`self.InheritLateralVelocity`)) (* (.z (`KismetMathLibrary.InverseTransformDirection` _output_get (`self.GetVelocity` _instigator))) _inheritvelocity)))))
    (:`else`
      (return (0.0 0.0 0.0)))))

(fn `CalculateLaunchImpulse`
  (returns (Result :type "Vector Structure"))
  (return (* (`self.LaunchDirection`) (`self.LaunchSpeed`))))

(fn `GetOwnerMaterialParams`
  (params (OwningWeapon :type "/Game/WeaponKit/Blueprints/Classes/BP_WeaponActorBase_WK Object Reference"))
  (returns (MaterialInst :type "MaterialInstance Object Reference") (ColorParam :type Name) (Color :type "LinearColor Structure"))
  (bind ((`SkinType_2_6CDCF899435CF19A593C24B16720FF40` _skintype) (`SkinColor_5_F8C2FF134EF6D5DC864EB08A5135BEF6` _skincolor)) (break `/Game/WeaponKit/Blueprints/Classes/FWeaponSettings_WK` (`/Game/WeaponKit/Blueprints/Classes/BP_WeaponActorBase_WK.Settings` OwningWeapon)))
  (return (`/Game/WeaponKit/Blueprints/Classes/BPFL_WeaponKitUtils.GetMaterialInstForSkinType` _skintype (`/Game/WeaponKit/Blueprints/Classes/BP_WeaponActorBase_WK.MaterialInstances` OwningWeapon)) "Color" _skincolor))

(fn `GetOwningWeapon`
  (returns (Weapon :type "/Game/WeaponKit/Blueprints/Classes/BP_WeaponActorBase_WK Object Reference"))
  (bind _asbp_weapon_actor_base_wk (cast `/Game/WeaponKit/Blueprints/Classes/BP_WeaponActorBase_WK` (`self.GetOwner`))
    (:`then`
      (return _asbp_weapon_actor_base_wk))
    (:`CastFailed`
      (return null))))

(fn `PlayLaunchSound`
  (bind _launchsound (`self.LaunchSound`)
    (:`then`
      (`GameplayStatics.PlaySoundAtLocation` _launchsound (`self.K2_GetActorLocation`) (struct) 1.0 1.0 0.0 "/Game/WeaponKit/FX/SA_Default_WK.SA_Default_WK" null self))
    (:`else`)))

(fn `UserConstructionScript`)