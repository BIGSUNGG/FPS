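; Base gun actor for the weapon kit, extending a parent weapon class with muzzle, magazine, pointer and scope attachments.
; The construction script attaches each part to named sockets on the body mesh, and getters expose these parts and the pointer laser mesh.
; FOV material setup calls the parent, then enlarges scope, muzzle and laser bounds scale when FOV materials are present.
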(fn `GetMagazineMesh`
  (returns (Mesh :type "StaticMeshComponent Object Reference"))
  (return (`self.MagazineMesh`)))

(fn `GetMuzzleMesh`
  (returns (Mesh :type "StaticMeshComponent Object Reference"))
  (return (`self.MuzzleMesh`)))

(fn `GetPointerLaserMesh`
  (returns (Mesh :type "StaticMeshComponent Object Reference"))
  (return (`self.PointerLaserMesh`)))

(fn `GetPointerMesh`
  (returns (Mesh :type "StaticMeshComponent Object Reference"))
  (return (`self.PointerMesh`)))

(fn `GetScopeMesh`
  (returns (Mesh :type "StaticMeshComponent Object Reference"))
  (return (`self.ScopeMesh`)))

(fn `SetupWeaponFovMaterials`
  (params (WeaponMainMat :type "MaterialInterface Object Reference") (WeaponColorSelectMat :type "MaterialInterface Object Reference") (WeaponGlassMat :type "MaterialInterface Object Reference") (WeaponScreenMat :type "MaterialInterface Object Reference") (WeaponLaserMat :type "MaterialInterface Object Reference") (BulletMat :type "MaterialInterface Object Reference"))
  (`parent.SetupWeaponFovMaterials` WeaponMainMat WeaponColorSelectMat WeaponGlassMat WeaponScreenMat WeaponLaserMat BulletMat)
  (if (`self.HasFovMaterials`)
    (`PrimitiveComponent.SetBoundsScale` (`self.ScopeMesh`) 4.0)
    (`PrimitiveComponent.SetBoundsScale` (`self.MuzzleMesh`) 4.0)
    (`PrimitiveComponent.SetBoundsScale` (`self.PointerLaserMesh`) 4.0)))

(fn `UserConstructionScript`
  (`/Game/WeaponKit/Blueprints/Classes/BPFL_WeaponKitUtils.AttachMuzzle` (`self.GetBodyMesh`) (`self.MuzzleMesh`))
  (`/Game/WeaponKit/Blueprints/Classes/BPFL_WeaponKitUtils.AttachMagazine` (`self.GetBodyMesh`) (`self.MagazineMesh`))
  (`/Game/WeaponKit/Blueprints/Classes/BPFL_WeaponKitUtils.AttachPointer` (`self.GetBodyMesh`) (`self.PointerMesh`))
  (`/Game/WeaponKit/Blueprints/Classes/BPFL_WeaponKitUtils.AttachScope` (`self.GetBodyMesh`) (`self.ScopeMesh`))
  (`parent.UserConstructionScript`))