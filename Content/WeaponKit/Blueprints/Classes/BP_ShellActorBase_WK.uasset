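; Base actor for an ejected weapon shell casing that simulates physics, tints its mesh and destroys itself after an optional lifetime.
; On BeginPlay, a physics-enabled shell with eject force gets a directional impulse with random scatter, a random spin and part of the instigator's velocity.
; If an FOV material is set, it replaces the mesh material using the shell material's parameters; either path applies the shell color.
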(event `self.ReceiveBeginPlay`
  (`|ExecutionSequence`
    (:`then_0`
      ;[1 1 1] Physics
      (`PrimitiveComponent.SetSimulatePhysics` (`self.ShellMesh`) (`self.bSpawnWithPhysics`))
      (if (and (`self.bSpawnWithPhysics`) (> (`self.EjectForce`) 0.01))
        (bind _output_get (set `self.EjectForceVec` (`self.CalculateEjectImpulse`)))
        (`PrimitiveComponent.AddImpulse` (`self.ShellMesh`) _output_get "None" false)
        (`PrimitiveComponent.AddAngularImpulseInDegrees` (`self.ShellMesh`) (`self.CalculateEjectAngularImpulse`) "None" false)
        (bind _instigator (`self.Instigator`)
          (:`then`
            (`PrimitiveComponent.SetPhysicsLinearVelocity` (`self.ShellMesh`) (* (`self.GetVelocity` _instigator) (`KismetMathLibrary.FClamp` (`self.InheritVelocity`))) true "None"))
          (:`else`))))
    (:`then_1`
      ;[1 1 1] Visuals
      (bind _output_get_2 (set `self.bHasFovMaterial` (`KismetSystemLibrary.IsValid` (`self.FovMaterial`))))
      (if _output_get_2
        (`self.ApplyFovMaterials`)
        (else
          (`MeshComponent.SetVectorParameterValueOnMaterials` (`self.ShellMesh`) "BulletColor" (`KismetMathLibrary.Conv_LinearColorToVector` (`self.ShellColor`))))))
    (:`then_2`
      ;[1 1 1] Lifetime
      (if (> (`self.Lifetime`) 0.01)
        (bind _returnvalue (`KismetSystemLibrary.K2_SetTimerDelegate` (delegate `OnLifetimeEnd`) (`self.Lifetime`) false 0.1))
        (set `self.LifetimeTimerHandle` _returnvalue)))))

(event `OnLifetimeEnd`
  ;[1 1 1] Lifetime
  (`self.K2_DestroyActor`))

(fn `ApplyFovMaterials`
  (if (`self.bHasFovMaterial`)
    (bind _newmatinstance (`/Game/WeaponKit/Blueprints/Classes/BPFL_WeaponKitUtils.SwapMeshMatWithParamsOf` (`self.ShellMesh`) 0 (`self.FovMaterial`) (`self.ShellMaterial`)))
    (`MaterialInstanceDynamic.SetVectorParameterValue` _newmatinstance "BulletColor" (`self.ShellColor`))))

(fn `CalculateEjectAngularImpulse`
  (returns (ReturnValue :type "Vector Structure"))
  (locals (RotateRand :type "Float (double-precision)" :default 0.0))
  (bind _rotaterand (`local.RotateRand`))
  (set `local.RotateRand` (`KismetMathLibrary.RandomFloatInRange` 9.0 16.0))
  (return (* (`KismetMathLibrary.TransformDirection` (`SceneComponent.K2_GetComponentToWorld` (`self.ShellMesh`)) (`KismetMathLibrary.MakeVector` 0.0 (* (`KismetMathLibrary.SelectFloat` _rotaterand (* _rotaterand -1.0) (`KismetMathLibrary.RandomBool`)) (`self.EjectRotateForce`)))) (`self.EjectRotateForce`))))

(fn `CalculateEjectImpulse`
  (returns (Result :type "Vector Structure"))
  (return (+ (* (`KismetMathLibrary.TransformDirection` (`SceneComponent.K2_GetComponentToWorld` (`self.ShellMesh`)) (`KismetMathLibrary.Normal` (`self.EjectDirection`) 0.01)) (* (`self.EjectForce`) 0.5)) (* (`KismetMathLibrary.RandomUnitVector`) (`self.RandForce`)))))

(fn `UserConstructionScript`)