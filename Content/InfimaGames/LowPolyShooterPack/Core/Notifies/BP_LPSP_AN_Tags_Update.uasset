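; An animation notify in the Low Poly Shooter Pack that updates the owning actor's ability tags during an animation.
; When fired, it gets the mesh owner's tag container through a message call, adds each configured tag, removes each configured tag, then sends the container back.
; It displays as "[LPSP] Update Tags".
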(fn `GetNotifyName`
  (returns (ReturnValue :type String))
  (return "[LPSP] Update Tags"))

(fn `Received_Notify`
  (params (MeshComp :type "SkeletalMeshComponent Object Reference") (Animation :type "AnimSequenceBase Object Reference"))
  (returns (ReturnValue :type Boolean))
  (locals (`Ability Tags` :type "GameplayTagContainer Structure"))
  (`|ExecutionSequence`
    (:`then_0`
      (`/Engine/EditorBlueprintResources/StandardMacros.IsValid` (`local.MeshComp`)
        (:`Is Valid`
          (bind _returnvalue (message `/Game/InfimaGames/LowPolyShooterPack/Core/Characters/BPI_LPSP_PCH.LPSP - Get Ability Tags` (`ActorComponent.GetOwner` (`local.MeshComp`))))
          (set `local.Ability Tags` _returnvalue)
          ;[0.8516 0 1 1 12] Add Tags
          (for _array_element (`BlueprintGameplayTagLibrary.BreakGameplayTagContainer` (`self.Tags Added`))
            (`BlueprintGameplayTagLibrary.AddGameplayTag` (`local.Ability Tags`) _array_element))
          ;[1 0 0.4453 1 12] Remove Tags
          (for _array_element_2 (`BlueprintGameplayTagLibrary.BreakGameplayTagContainer` (`self.Tags Removed`))
            (`BlueprintGameplayTagLibrary.RemoveGameplayTag` (`local.Ability Tags`) _array_element_2))
          (message `/Game/InfimaGames/LowPolyShooterPack/Core/Characters/BPI_LPSP_PCH.LPSP - On Set Ability Tags` (`ActorComponent.GetOwner` (`local.MeshComp`)) (`local.Ability Tags`)))))
    (:`then_1`
      (return true))))