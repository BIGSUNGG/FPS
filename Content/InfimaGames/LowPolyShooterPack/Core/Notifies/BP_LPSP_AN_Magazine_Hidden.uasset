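; Anim notify in the Low Poly Shooter Pack that sets magazine visibility during animations, shown in the editor as "Set Magazine Hidden".
; When fired, it sends the Hidden value to the mesh component's owner, if valid, through an LPSP message call, leaving the actual hiding to that actor.
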(fn `GetNotifyName`
  (returns (ReturnValue :type String))
  (return "Set Magazine Hidden"))

(fn `Received_Notify`
  (params (MeshComp :type "SkeletalMeshComponent Object Reference") (Animation :type "AnimSequenceBase Object Reference"))
  (returns (ReturnValue :type Boolean))
  (locals (`Actor Weapon` :type "Actor Object Reference"))
  (`|ExecutionSequence`
    (:`then_0`
      (`/Engine/EditorBlueprintResources/StandardMacros.IsValid` (`ActorComponent.GetOwner` (`local.MeshComp`))
        (:`Is Valid`
          (message `/Game/InfimaGames/LowPolyShooterPack/Core/Weapons/BPI_LPSP_WEP.LPSP - On Set Hidden Magazine` (`ActorComponent.GetOwner` (`local.MeshComp`)) (`self.Hidden`)))))
    (:`then_1`
      (return true))))