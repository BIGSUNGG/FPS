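; Animation notify from the Low Poly Shooter Pack that shows or hides the reserve magazine of the equipped weapon during an animation.
; When triggered, it asks the mesh owner for its equipped item and passes its Visibility variable to that weapon through a set-visibility message.
; Validity checks guard both the owner and the weapon, and the notify displays as "Set Reserve Magazine Visibility".
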(fn `GetNotifyName`
  (returns (ReturnValue :type String))
  (return "Set Reserve Magazine Visibility"))

(fn `Received_Notify`
  (params (MeshComp :type "SkeletalMeshComponent Object Reference") (Animation :type "AnimSequenceBase Object Reference"))
  (returns (ReturnValue :type Boolean))
  (locals (`Actor Weapon` :type "Actor Object Reference"))
  (`|ExecutionSequence`
    (:`then_0`
      (`/Engine/EditorBlueprintResources/StandardMacros.IsValid` (`ActorComponent.GetOwner` (`local.MeshComp`))
        (:`Is Valid`
          (bind _equipped_item (message `/Game/InfimaGames/LowPolyShooterPack/Core/Characters/BPI_LPSP_PCH.LPSP - Get Equipped Item` (`ActorComponent.GetOwner` (`local.MeshComp`))))
          (bind _output_get (set `local.Actor Weapon` _equipped_item))
          (`/Engine/EditorBlueprintResources/StandardMacros.IsValid` _output_get
            (:`Is Valid`
              (message `/Game/InfimaGames/LowPolyShooterPack/Core/Weapons/BPI_LPSP_WEP.Set Reserve Magazine Visibility` (`local.Actor Weapon`) (`self.Visibility`)))))))
    (:`then_1`
      (return true))))