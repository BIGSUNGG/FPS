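; Anim notify state from the Low Poly Shooter Pack that sets magazine visibility on a character's equipped item during an animation.
; On every notify tick it gets the equipped item from the mesh's owner and passes its Hidden value to that item through a message.
; It applies the value only on tick, with no begin or end handling, and skips invalid owners or items.
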(fn `GetNotifyName`
  (returns (ReturnValue :type String))
  (return "[Character] Hide Magazine"))

(fn `Received_NotifyTick`
  (params (MeshComp :type "SkeletalMeshComponent Object Reference") (Animation :type "AnimSequenceBase Object Reference") (FrameDeltaTime :type "Float (double-precision)"))
  (returns (ReturnValue :type Boolean))
  (`/Engine/EditorBlueprintResources/StandardMacros.IsValid` (`ActorComponent.GetOwner` (`local.MeshComp`))
    (:`Is Valid`
      (bind _equipped_item (message `/Game/InfimaGames/LowPolyShooterPack/Core/Characters/BPI_LPSP_PCH.LPSP - Get Equipped Item` (`ActorComponent.GetOwner` (`local.MeshComp`))))
      (`/Engine/EditorBlueprintResources/StandardMacros.IsValid` _equipped_item
        (:`Is Valid`
          (message `/Game/InfimaGames/LowPolyShooterPack/Core/Weapons/BPI_LPSP_WEP.LPSP - On Set Hidden Magazine` _equipped_item (`self.Hidden`))
          (return true))))))