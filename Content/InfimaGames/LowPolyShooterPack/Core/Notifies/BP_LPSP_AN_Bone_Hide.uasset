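; Animation notify in the Low Poly Shooter Pack that hides or shows a named bone on the animated mesh.
; When the notify fires, a Hidden flag selects between hiding the bone with its physics body terminated and unhiding it.
; It displays as "Hide Bone" in the animation timeline.
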(fn `GetNotifyName`
  (returns (ReturnValue :type String))
  (return "Hide Bone"))

(fn `Received_Notify`
  (params (MeshComp :type "SkeletalMeshComponent Object Reference") (Animation :type "AnimSequenceBase Object Reference"))
  (returns (ReturnValue :type Boolean))
  (`|ExecutionSequence`
    (:`then_0`
      (if (`self.Hidden`)
        (`SkinnedMeshComponent.HideBoneByName` (`local.MeshComp`) (`self.Bone Name`) "PBO_Term")
        (else
          (`SkinnedMeshComponent.UnHideBoneByName` (`local.MeshComp`) (`self.Bone Name`)))))
    (:`then_1`
      (return true))))