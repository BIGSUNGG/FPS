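; Base laser Blueprint for Low Poly Shooter Pack weapons that tracks whether the laser is visible.
; EnableLaser and DisableLaser change the Visible flag only when its state differs.
; Visible has a RepNotify that, like BeginPlay, calls UpdateVisible.
; UpdateVisible is empty here, so this Blueprint holds the state logic without any visual response of its own.
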(event `/Game/InfimaGames/LowPolyShooterPack/Core/Weapons/BPI_LPSP_WEP_Laser.Enable Laser`
  (if (not (`self.Visible`))
    (set `self.Visible` true)))

(event `/Game/InfimaGames/LowPolyShooterPack/Core/Weapons/BPI_LPSP_WEP_Laser.Disable Laser`
  (if (`self.Visible`)
    (set `self.Visible` false)))

(event `Event Update Visible`)

(event `self.ReceiveBeginPlay`
  (`parent.ReceiveBeginPlay`)
  (`self.Event Update Visible`))

(fn `OnRep_Visible`
  (`self.Event Update Visible`))

(fn `UserConstructionScript`
  (`parent.UserConstructionScript`))